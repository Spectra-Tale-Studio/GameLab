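; Base enemy character that supplies movement helpers and attack requests for enemies moving along the X axis.
; GetDestination offsets the actor's location by a distance times Direction, which ReverseDirection flips.
; JumptoDestination launches the character on a suggested projectile arc toward a raised target, using only its X and Z.
; Attack requests switch ActionState, with the start also jumping the animation to Attack; debug prints remain.
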(event EventBeginPlay
  (|CallParentFunction) ; This node is disabled and will not be called.\nDrag off pins to build functionality.
)

(event Collision|EventActorBeginOverlap
  (params (OtherActor :type Actor%20Object%20Reference))
  (|CallParentFunction OtherActor) ; This node is disabled and will not be called.\nDrag off pins to build functionality.
)

(event EventTick
  (params (DeltaSeconds :type Float%20%28single-precision%29))
  (|CallParentFunction DeltaSeconds) ; This node is disabled and will not be called.\nDrag off pins to build functionality.
)

(event EventJumptoDestination
  (params (Destination :type Vector :default "0, 0, 0"))
  (bind (_x _y _z) (Math|Vector|BreakVector Destination))
  (bind _outlaunchvelocity (Game|SuggestProjectileVelocityCustomArc (Transformation|GetActorLocation) (Math|Vector|MakeVector _x 0.0 (+ _z 2.5e+02)) 0.0 0.5))
  (Character|LaunchCharacter _outlaunchvelocity false false)
  (Development|PrintString "Hello"))

(event EventRequestAttack
  (Variables|Default|SetActionState "NewEnumerator2")
  (CallFunction|ChangeAnim "Attack" "None"))

(event EventRequestEndAttack
  (Variables|Default|SetActionState "NewEnumerator0"))

(fn ConstructionScript
  (|CallParentFunction))

(fn GetDestination
  (params (Distance :type Float%20%28double-precision%29))
  (bind _returnvalue (Transformation|GetActorLocation))
  (bind _direction (Variables|Default|GetDirection))
  (bind _returnvalue_2 (* Distance _direction))
  (bind _returnvalue_3 (+ _returnvalue (Math|Vector|MakeVector _returnvalue_2 0.0 0.0)))
  (return (Math|Vector|MakeVector (.x _returnvalue_3) (.y _returnvalue_3) 0.0)))

(fn ReverseDirection
  (Variables|Default|SetDirection (* (Variables|Default|GetDirection) -1.0))
  (Development|PrintString "Reverse - dio porco"))