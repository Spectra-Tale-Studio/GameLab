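; Base PaperZD character that handles X-axis movement, damage reactions, death and revival.
; Damage events forward hit data to the health component, whose callbacks set the action state and jump animation nodes.
; Getting hurt sets an invulnerability flag until RequestEndHurt clears it.
; Move, dash, attack, jump and interact checks share one gate: control flag, allowed movement modes and blocked action states; only movement is implemented here.
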(event OnDeath(BP_HealthComponent)
  (Variables|RuntimeState|SetActionState "NewEnumerator5")
  (CallFunction|ChangeAnim "Death" "None"))

(event OnRevived(BP_HealthComponent)
  (params (CurrentHealth :type Float%20%28double-precision%29))
  (Variables|RuntimeState|SetActionState "NewEnumerator0")
  (CallFunction|ChangeAnim "Revive" "None"))

(event OnDamaged(BP_HealthComponent)
  (Variables|RuntimeState|SetActionState "NewEnumerator4")
  (CallFunction|ChangeAnim "Damage" "None")
  (Variables|Default|SetbInvulnerability true))

(event EventBeginPlay)

(event Collision|EventActorBeginOverlap
  (params (OtherActor :type Actor%20Object%20Reference)))

(event EventTick
  (params (DeltaSeconds :type Float%20%28single-precision%29)))

(event EventRequestMove
  (params (MoveValue :type Vector%202D%20Structure))
  (bind _x (Math|Vector2D|BreakVector2D MoveValue))
  (bind _returnvalue (CallFunction|CanMove))
  (if _returnvalue
    (Pawn|Input|AddMovementInput "1.000000,0.000000,0.000000" _x false)
    (Variables|Runtimestate|SetFacingDirection _x)
    (Variables|RuntimeState|SetMoveInputValue MoveValue)))

(event Game|Damage|EventPointDamage
  (params (Damage :type Float%20%28single-precision%29) (DamageType :type Damage%20Type%20Object%20Reference) (HitLocation :type Vector :default "0, 0, 0") (HitNormal :type Vector :default "0, 0, 0") (HitComponent :type Primitive%20Component%20Object%20Reference) (BoneName :type Name :default "None") (ShotFromDirection :type Vector :default "0, 0, 0") (InstigatedBy :type Controller%20Object%20Reference) (DamageCauser :type Actor%20Object%20Reference) (HitInfo :type Hit%20Result%20Structure%20%28by%20ref%29))
  ;[0.15 0 0.009812 0.5] Damage
  (Default|ApplyDamage (Variables|Default|GetBP_HealthComponent) (Utilities|Struct|MakeST_DamageData Damage DamageCauser InstigatedBy HitLocation HitNormal 0.0)))

(event Game|Damage|EventRadialDamage
  (params (DamageReceived :type Float%20%28single-precision%29) (DamageType :type Damage%20Type%20Object%20Reference) (Origin :type Vector :default "0, 0, 0") (HitInfo :type Hit%20Result%20Structure%20%28by%20ref%29) (InstigatedBy :type Controller%20Object%20Reference) (DamageCauser :type Actor%20Object%20Reference))
  ;[0.15 0 0.009812 0.5] Damage
  (Default|ApplyDamage (Variables|Default|GetBP_HealthComponent) (Utilities|Struct|MakeST_DamageData DamageReceived DamageCauser InstigatedBy "0.000000,0.000000,0.000000" "0.000000,0.000000,0.000000" 0.0)))

(event Game|Damage|EventAnyDamage
  (params (Damage :type Float%20%28single-precision%29) (DamageType :type Damage%20Type%20Object%20Reference) (InstigatedBy :type Controller%20Object%20Reference) (DamageCauser :type Actor%20Object%20Reference))
  (bind _returnvalue (Transformation|GetActorLocation))
  ;[0.15 0 0.009812 0.5] Damage
  (Default|ApplyDamage (Variables|Default|GetBP_HealthComponent) (Utilities|Struct|MakeST_DamageData Damage DamageCauser InstigatedBy _returnvalue (Math|Vector|Normalize (- _returnvalue (Transformation|GetActorLocation DamageCauser))) 0.0)))

(event EventRequestEndHurt
  (Variables|RuntimeState|SetActionState "NewEnumerator0")
  (Variables|Default|SetbInvulnerability false))

(fn ConstructionScript)

(fn CanMove
  (return (Math|Boolean|ANDBoolean (Variables|RuntimeState|GetbCanReceiveControlRequests) (Utilities|Array|ContainsItem (Variables|Movepermission|GetMoveAllowedMovementModes) (Variables|/Script/Engine.CharacterMovementComponent|GetMovementMode (Variables|Character|GetCharacterMovement))) (not (Utilities|Array|ContainsItem (Variables|MovePermission|GetMoveBlockedActionStates) (Variables|RuntimeState|GetActionState))))))

(fn CanDash
  (return (Math|Boolean|ANDBoolean (Variables|RuntimeState|GetbCanReceiveControlRequests) (Utilities|Array|ContainsItem (Variables|Dashpermission|GetDashAllowedMovementModes) (Variables|/Script/Engine.CharacterMovementComponent|GetMovementMode (Variables|Character|GetCharacterMovement))) (not (Utilities|Array|ContainsItem (Variables|Dashpermission|GetDashBlockedActionStates) (Variables|RuntimeState|GetActionState))))))

(fn CanAttack
  (return (Math|Boolean|ANDBoolean (Variables|RuntimeState|GetbCanReceiveControlRequests) (Utilities|Array|ContainsItem (Variables|Attackpermission|GetAttackAllowedMovementModes) (Variables|/Script/Engine.CharacterMovementComponent|GetMovementMode (Variables|Character|GetCharacterMovement))) (not (Utilities|Array|ContainsItem (Variables|AttackPermission|GetAttackBlockedActionStates) (Variables|RuntimeState|GetActionState))))))

(fn CanJumpInternal
  (return (Math|Boolean|ANDBoolean (Variables|RuntimeState|GetbCanReceiveControlRequests) (Utilities|Array|ContainsItem (Variables|Jumppermission|GetJumpAllowedMovementModes) (Variables|/Script/Engine.CharacterMovementComponent|GetMovementMode (Variables|Character|GetCharacterMovement))) (not (Utilities|Array|ContainsItem (Variables|JumpPermission|GetJumpBlockedActionStates) (Variables|RuntimeState|GetActionState))))))

(fn CanInteract
  (return (Math|Boolean|ANDBoolean (Variables|RuntimeState|GetbCanReceiveControlRequests) (Utilities|Array|ContainsItem (Variables|Interactpermission|GetInteractAllowedMovementModes) (Variables|/Script/Engine.CharacterMovementComponent|GetMovementMode (Variables|Character|GetCharacterMovement))) (not (Utilities|Array|ContainsItem (Variables|InteractPermission|GetInteractBlockedActionStates) (Variables|RuntimeState|GetActionState))))))

(fn ChangeAnim
  (params (JumpName%20 :type Name) (StateMachineName :type Name))
  (Class|PaperZDAnimInstance|JumptoNode (Variables|/Script/PaperZD.PaperZDAnimationComponent|GetAnimInstance (Variables|Default|GetAnimationComponent)) JumpName%20 StateMachineName))

(fn CanbeDamaged
  (return (not (Variables|Default|GetbInvulnerability))))