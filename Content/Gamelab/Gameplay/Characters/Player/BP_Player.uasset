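; Player character Blueprint for a sprite-based game, handling jump, multi-jump, unlockable dash, attack and interact requests.
; Requests pass parent and local Can checks, then set ActionState and, for dash and attack, jump animation states.
; Dash zeroes gravity, friction and braking, sweeps the actor along FacingDirection with a timeline lerp, then restores them.
; Landing resets the jump count; landing or leaving walking calls SetLastSafeLocation, which only records while not falling.
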(event EventBeginPlay
  (|CallParentFunction)
  (CallFunction|SetMaxAvailableJumps (Variables|Jump|GetMaxAvailableJumps))
  (Components|Timeline|SetTimelineLength (Variables|Default|GetDash) (Variables|Dash|GetDashDuration)))

(event Collision|EventActorBeginOverlap
  (params (OtherActor :type Actor%20Object%20Reference))
  (|CallParentFunction OtherActor) ; This node is disabled and will not be called.\nDrag off pins to build functionality.
)

(event EventRequestEndAttack
  ;[0.15 0.12 0.01915 0.5] Attack
  (Variables|Default|SetActionState "NewEnumerator0"))

(event EventTick
  (params (DeltaSeconds :type Float%20%28single-precision%29))
  (|CallParentFunction DeltaSeconds)
  (Development|PrintText (Utilities|Text|FormatText "Movement: {0} 
State: {1} 
" (Utilities|String|EnumtoString (Variables|/Script/Engine.CharacterMovementComponent|GetMovementMode (Variables|Character|GetCharacterMovement))) (Utilities|String|EnumtoString (Variables|Default|GetActionState))) true true "(R=0.000000,G=0.660000,B=1.000000,A=1.000000)" 2.0 "caharacterstate"))

(event EventRequestStopJump
  (Character|StopJumping))

(event EventOnMovementModeChanged
  (params (PrevMovementMode :type EMovementMode%20Enum :default "MOVE_None") (NewMovementMode :type EMovementMode%20Enum :default "MOVE_None") (PrevCustomMode :type Byte :default 0) (NewCustomMode :type Byte :default 0))
  (if (and (Utilities|Enum|Equal(Enum) PrevMovementMode "MOVE_Walking") (Utilities|Enum|Equal(Enum) NewMovementMode "MOVE_Falling"))
    (CallFunction|SetLastSafeLocation)))

(event EventRequestInteract
  (bind _returnvalue (CallFunction|CanInteract))
  (if _returnvalue
    (Variables|Default|SetActionState "NewEnumerator3")
    (Default|CheckOverlap (Variables|Default|GetBP_Interactor))
    (Variables|Default|SetActionState "NewEnumerator0")))

(event EventRequestDash
  (bind _charactermovement (Variables|Character|GetCharacterMovement))
  (bind _charactermovement_2 (Variables|Character|GetCharacterMovement))
  ;[0.15 0.02844 0 0.5] Dash
  (bind _returnvalue (CallFunction|CanDash))
  (if _returnvalue
    (Variables|Default|SetActionState "NewEnumerator1")
    (Variables|Dash|SetCachedGravityScale (Variables|/Script/Engine.CharacterMovementComponent|GetGravityScale _charactermovement_2))
    (Variables|/Script/Engine.CharacterMovementComponent|SetGravityScale _charactermovement_2 0.0)
    (Variables|Dash|SetCachedGroundFriction (Variables|/Script/Engine.CharacterMovementComponent|GetGroundFriction _charactermovement_2))
    (Variables|/Script/Engine.CharacterMovementComponent|SetGroundFriction _charactermovement_2 0.0)
    (Variables|Dash|SetCachedBrakingDecelerationWalking (Variables|/Script/Engine.CharacterMovementComponent|GetBrakingDecelerationWalking _charactermovement_2))
    (Variables|/Script/Engine.CharacterMovementComponent|SetBrakingDecelerationWalking _charactermovement_2 0.0)
    (bind _output_get (Variables|Dash|SetDashDirection (Math|Vector|MakeVector (Variables|Default|GetFacingDirection) 0.0 0.0)))
    (bind _output_get_2 (Variables|Dash|SetDashStartLocation (Transformation|GetActorLocation)))
    (Variables|Dash|SetDashTargetLocation (+ _output_get_2 (* _output_get (* (Variables|Dash|GetDashDistance) 1e+03))))
    (CallFunction|ChangeAnim "Dash" "None")
    (bind _alpha (Timeline|Dash PlayFromStart)
      (:Update
        (Transformation|SetActorLocation (Math|Vector|Lerp(Vector) (Variables|Dash|GetDashStartLocation) (Variables|Dash|GetDashTargetLocation) _alpha) true false))
      (:Finished
        (Components|Movement|StopMovementImmediately _charactermovement)
        (Variables|/Script/Engine.CharacterMovementComponent|SetGravityScale _charactermovement (Variables|Dash|GetCachedGravityScale))
        (Variables|/Script/Engine.CharacterMovementComponent|SetGroundFriction _charactermovement (Variables|Dash|GetCachedGroundFriction))
        (Variables|/Script/Engine.CharacterMovementComponent|SetBrakingDecelerationWalking _charactermovement (Variables|Dash|GetCachedBrakingDecelerationWalking))
        (Variables|Default|SetActionState "NewEnumerator0")))))

(event EventRequestAttack
  ;[0.15 0.12 0.01915 0.5] Attack
  (bind _returnvalue (CallFunction|CanAttack))
  (if _returnvalue
    (Variables|Attack|SetLastAttackTime (+ (Utilities|Time|GetGameTimeinSeconds) (Variables|Attack|GetAttackRatio)))
    (Variables|Default|SetActionState "NewEnumerator2")
    (Variables|Attack|SetbAttackWasStartedInAir (AI|Components|NavMovement|IsFalling (Variables|Character|GetCharacterMovement)))
    (CallFunction|ChangeAnim "Attack" "None")))

(event EventOnLanded
  (params (Hit :type Hit%20Result%20Structure%20%28by%20ref%29))
  (Variables|Jump|SetUsedJumps 0)
  (CallFunction|SetLastSafeLocation))

(event EventRequestJump
  (if (Character|CanJump)
    (Character|Jump)
    (Math|Integer|IncrementInt (Variables|Jump|GetUsedJumps))))

(fn ConstructionScript
  (|CallParentFunction))

(fn SetMaxAvailableJumps
  (params (MaxAvailableJumps :type Integer))
  (if (>= MaxAvailableJumps 0)
    (bind _output_get (Variables|Jump|SetMaxAvailableJumps MaxAvailableJumps))
    (Variables|Default|SetJumpMaxCount (+ _output_get 1))))

(fn SetLastSafeLocation
  (if (not (AI|Components|NavMovement|IsFalling (Variables|Character|GetCharacterMovement)))
    (Variables|SafeLoaction|SetLastSafeLocation (Math|Transform|MakeTransform (+ (Transformation|GetActorLocation) (Variables|SafeLoaction|GetOffsetLastSafeLocation)) (Transformation|GetActorRotation) "1.000000,1.000000,1.000000"))))

(fn CanJumpInternal
  (bind _returnvalue (|CallParentFunction))
  (return (and _returnvalue (>= (Variables|Jump|GetMaxAvailableJumps) (Variables|Jump|GetUsedJumps)))))

(fn CanAttack
  (bind _returnvalue (|CallParentFunction))
  (return (and _returnvalue (> (Utilities|Time|GetGameTimeinSeconds) (Variables|Attack|GetLastAttackTime)))))

(fn CanDash
  (bind _returnvalue (|CallParentFunction))
  (return (and _returnvalue (Variables|Dash|GetDashUnlock))))

(fn AttackDamageValue
  (return (Variables|Attack|GetAttackDamage)))

(fn AttackRadiusValue
  (return (Variables|Attack|GetAttackRadius)))

(fn GetSpriteComponent
  (return (Variables|Default|GetSprite)))

(fn KnockbackDirectionValue
  (return (* (* (Math|Vector|Normalize (Variables|Attack|GetKnockbackDirection)) (Math|Vector|MakeVector (Variables|Default|GetFacingDirection) 1.0 1.0)) (Variables|Attack|GetKnockbackForce))))