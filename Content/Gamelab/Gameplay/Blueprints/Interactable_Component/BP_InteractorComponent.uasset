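; Interactor component that finds the closest BP_InteractableBase actor around it and triggers its interaction.
; CheckOverlap, not called within this graph, runs a WorldDynamic sphere overlap, compares distances from the owner and calls InteractMessage on NearestActor.
; NearestActor is never cleared here, so its previous value competes in each search.
; Tick draws the search sphere when the debug check passes, and debug strings report the result.
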(event EventBeginPlay)

(event EventTick
  (params (DeltaSeconds :type Float%20%28single-precision%29))
  (Variables|Debug|GetbEnableDebugDraw
    (:then
      (CallFunction|DrawDebug))
    (:else)))

(fn CheckOverlap
  (bind (_outactors _returnvalue) (Collision|SphereOverlapActors (Transformation|GetWorldLocation) (Variables|Default|GetSphereRadius) (Utilities|Array|MakeArray "ObjectTypeQuery2") "/Game/Gamelab/Gameplay/Blueprints/Interactables/BP_InteractableBase.BP_InteractableBase_C"))
  (if _returnvalue
    (LocalVariables|SetActorLocationRef (.location (Transformation|GetActorTransform (Components|GetOwner))))
    (for _array_element _outactors
      (bind _nearestactor (LocalVariables|GetNearestActor)
        (:then
          (if (> (Math|Vector|Distance(Vector) (LocalVariables|GetActorLocationRef) (.location (Transformation|GetActorTransform _nearestactor))) (Math|Vector|Distance(Vector) (LocalVariables|GetActorLocationRef) (.location (Transformation|GetActorTransform _array_element))))
            (LocalVariables|SetNearestActor _array_element)))
        (:else
          (LocalVariables|SetNearestActor _array_element))))
    (Class|BPIInteractable|Interact(Message) (LocalVariables|GetNearestActor))
    (Development|PrintString (Utilities|GetDisplayName (LocalVariables|GetNearestActor)))
    (else
      (Development|PrintString "nheeeeeeeeeeeeeeeeeessuno"))))

(fn DrawDebug
  (Rendering|Debug|DrawDebugSphere (Transformation|GetWorldLocation) (Variables|Default|GetSphereRadius) 12 "(R=1.000000,G=0.000000,B=0.000000,A=1.000000)" 0.0 3.0))