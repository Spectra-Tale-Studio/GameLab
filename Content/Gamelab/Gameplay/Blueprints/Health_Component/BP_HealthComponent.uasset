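; Health component that tracks an owner's current and max health, handling damage, healing, death and revival.
; ApplyDamage checks an invulnerability time and calls Kill at zero health, while Heal on a dead owner routes to Revive if allowed.
; Damage, heal, kill and revive each fire event dispatchers, then execute pluggable action objects that InitializeHealth constructs from configurable classes.
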(event EventBeginPlay)

(event EventTick
  (params (DeltaSeconds :type Float%20%28single-precision%29)))

(fn InitializeHealth
  (Variables|Default|SetRuntimeMaxHealth (Variables|Default|GetBaseMaxHealth))
  (Variables|Default|SetbIsDead%20 false)
  (Variables|Default|SetCachedOwner%20 (Components|GetOwner))
  (bind _damageactionclass (Variables|Default|GetDamageActionClass)
    (:then
      (bind _returnvalue (Game|ConstructObjectfromClass _damageactionclass))
      (Variables|Default|SetDamageActionInstance _returnvalue))
    (:else
      _))
  (bind _healactionclass (Variables|Default|GetHealActionClass)
    (:then
      (bind _returnvalue_2 (Game|ConstructObjectfromClass _healactionclass))
      (Variables|Default|SetHealActionInstance _returnvalue_2))
    (:else
      _))
  (bind _killactionclass (Variables|Default|GetKillActionClass)
    (:then
      (bind _returnvalue_3 (Game|ConstructObjectfromClass _killactionclass))
      (Variables|Default|SetKillActionInstance _returnvalue_3))
    (:else
      _))
  (bind _reviveactionclass (Variables|Default|GetReviveActionClass)
    (:then
      (bind _returnvalue_4 (Game|ConstructObjectfromClass _reviveactionclass))
      (Variables|Default|SetReviveActionInstance _returnvalue_4))
    (:else)))

(fn ApplyDamage
  (params (DamageData%20 :type ST%20Damage%20Data%20Structure))
  (bind _defaultinvulnerabilityduration_ (Variables|Default|GetDefaultInvulnerabilityDuration%20))
  (Variables|Default|GetbIsDead%20
    (:then)
    (:else
      (if (not (< (Utilities|Time|GetGameTimeinSeconds) (Variables|Default|GetInvulnerabilityEndTime%20)))
        (bind _output_get (Variables|Default|SetDamageData DamageData%20))
        (bind _output_get_2 (Variables|Default|SetCurrentHealth (Math|Float|Clamp(Float) (- (Variables|Default|GetCurrentHealth) (.DamageAmount (Utilities|Struct|BreakST_DamageData _output_get))) 0.0 (Variables|Default|GetRuntimeMaxHealth))))
        (if (<= _output_get_2 0.0)
          (CallFunction|Kill)
          (else
            (if (> _defaultinvulnerabilityduration_ 0.0)
              (Variables|Default|SetInvulnerabilityEndTime%20 _defaultinvulnerabilityduration_))
            (Default|CallOnDamaged)
            (Default|CallOnHealthChanged (Variables|Default|GetCurrentHealth) (Variables|Default|GetRuntimeMaxHealth))
            (Default|ExecuteAction (Variables|Default|GetDamageActionInstance) self)))))))

(fn Heal
  (params (HealData%20 :type ST%20Heal%20Data%20Structure))
  (bind _output_get (Variables|Default|SetHealData HealData%20))
  (Variables|Default|GetbIsDead%20
    (:then
      (Variables|Default|GetbCanBeRevive
        (:then
          (CallFunction|Revive (.HealAmount (Utilities|Struct|BreakST_HealData _output_get))))
        (:else)))
    (:else
      (Variables|Default|SetCurrentHealth (Math|Float|Clamp(Float) (+ (Variables|Default|GetCurrentHealth) (.HealAmount (Utilities|Struct|BreakST_HealData _output_get))) 0.0 (Variables|Default|GetRuntimeMaxHealth)))
      (Default|CallOnHealed)
      (Default|CallOnHealthChanged (Variables|Default|GetCurrentHealth) (Variables|Default|GetRuntimeMaxHealth))
      (Default|ExecuteAction (Variables|Default|GetHealActionInstance) self))))

(fn Kill
  (Variables|Default|GetbIsDead%20
    (:then)
    (:else
      (Variables|Default|SetCurrentHealth 0.0)
      (Variables|Default|SetbIsDead%20 true)
      (Default|CallOnDeath)
      (Default|CallOnHealthChanged (Variables|Default|GetCurrentHealth) (Variables|Default|GetRuntimeMaxHealth))
      (Default|ExecuteAction (Variables|Default|GetKillActionInstance) self))))

(fn Revive
  (params (ReviveHealth%20 :type Float%20%28double-precision%29))
  (Variables|Default|GetbIsDead%20
    (:then
      (bind _output_get (Variables|Default|SetCurrentHealth (Math|Float|Clamp(Float) ReviveHealth%20 0.0 (Variables|Default|GetRuntimeMaxHealth))))
      (Default|CallOnRevived _output_get)
      (Default|CallOnHealthChanged (Variables|Default|GetCurrentHealth) (Variables|Default|GetRuntimeMaxHealth))
      (Default|ExecuteAction (Variables|Default|GetReviveActionInstance) self))
    (:else)))

(fn ModifyMaxHealth
  (params (Delta%20 :type Float%20%28double-precision%29))
  (Variables|Default|SetRuntimeMaxHealth (Math|Float|Max(Float) (+ Delta%20 (Variables|Default|GetRuntimeMaxHealth)) 0.0))
  (Default|CallOnMaxHealthChanged 0.0))

(fn GetHealthPercent
  (bind _runtimemaxhealth (Variables|Default|GetRuntimeMaxHealth))
  (if (<= _runtimemaxhealth 0.0)
    (return 0.0)
    (else
      (return (/ (Variables|Default|GetCurrentHealth) _runtimemaxhealth)))))

(fn IsAlive
  (return (not (Variables|Default|GetbIsDead%20))))