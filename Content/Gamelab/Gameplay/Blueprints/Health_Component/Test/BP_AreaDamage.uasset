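; Test area-damage actor in the health component folder that repeatedly damages an actor while it overlaps the area.
; When no target is stored, an overlap stores the entering actor and starts a fast looping timer that applies fixed damage, so only one actor is affected at a time.
; An end-overlap handler bound at BeginPlay stops the timer and clears the target when that actor leaves.
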(event Custom|damage
  (Game|Damage|ApplyDamage (Variables|Default|GetOther%20Actor) 1e+01 0 self))

(event Custom|OnActorEndOverlap_Event
  (params (OverlappedActor :type Actor%20Object%20Reference) (OtherActor :type Actor%20Object%20Reference))
  (if (== OtherActor (Variables|Default|GetOther%20Actor))
    (Utilities|Time|ClearandInvalidateTimerbyHandle (Variables|Default|GetNewVar))
    (Variables|Default|SetOther%20Actor 0)))

(event Collision|EventActorBeginOverlap
  (params (OtherActor :type Actor%20Object%20Reference))
  (Variables|Default|GetOther%20Actor
    (:then)
    (:else
      (Variables|Default|SetOther%20Actor OtherActor)
      (bind _returnvalue (Utilities|Time|SetTimerbyEvent (delegate Custom|damage) 0.1 true))
      (Variables|Default|SetNewVar _returnvalue))))

(event EventBeginPlay
  (EventDispatchers|BindEventtoOnActorEndOverlap (delegate Custom|OnActorEndOverlap_Event)))

(fn ConstructionScript)