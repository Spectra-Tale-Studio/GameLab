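; Base Blueprint for saveable interactables whose activated state is tracked by ID in the game instance.
; Interact registers the actor's ID with the game instance, then calls InternalInteract.
; On BeginPlay, an ID that is already registered replays InternalInteract to restore the activated state without registering again.
; InternalInteract only calls its parent here, and GetGameData is an empty stub.
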(event EventBeginPlay
  (|CallParentFunction)
  (bind _returnvalue (Class|BPISaveActivatedID|ContaineActivatedIDs(Message) (Game|GetGameInstance) (Variables|Default|GetID)))
  (if _returnvalue
    (CallFunction|InternalInteract)))

(event Collision|EventActorBeginOverlap
  (params (OtherActor :type Actor%20Object%20Reference))
  (|CallParentFunction OtherActor) ; This node is disabled and will not be called.\nDrag off pins to build functionality.
)

(event EventTick
  (params (DeltaSeconds :type Float%20%28single-precision%29))
  (|CallParentFunction DeltaSeconds) ; This node is disabled and will not be called.\nDrag off pins to build functionality.
)

(event EventInteract
  (|CallParentFunction)
  (Class|BPISaveActivatedID|AddActivatedIDs(Message) (Game|GetGameInstance) (Variables|Default|GetID))
  (CallFunction|InternalInteract))

(event EventInternalInteract
  (|CallParentFunction))

(fn ConstructionScript
  (|CallParentFunction))

(fn GetGameData
  (return ""))