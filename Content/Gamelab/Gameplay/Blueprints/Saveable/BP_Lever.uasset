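; BP_Lever is an interactable lever that triggers a linked door.
; Interact calls the parent implementation, then plays a 2D interaction sound guarded by a DoOnce, while CanInteract always returns true.
; InternalInteract swaps the Paper2D sprite to its activated version and calls Receive on the referenced door.
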(event EventBeginPlay
  (|CallParentFunction) ; This node is disabled and will not be called.\nDrag off pins to build functionality.
)

(event Collision|EventActorBeginOverlap
  (params (OtherActor :type Actor%20Object%20Reference))
  (|CallParentFunction OtherActor) ; This node is disabled and will not be called.\nDrag off pins to build functionality.
)

(event EventTick
  (params (DeltaSeconds :type Float%20%28single-precision%29))
  (|CallParentFunction DeltaSeconds) ; This node is disabled and will not be called.\nDrag off pins to build functionality.
)

(event EventInteract
  (|CallParentFunction)
  (Utilities|FlowControl|DoOnce false
    (:Completed
      (Audio|PlaySound2D (Variables|Default|GetInteractSound) 1.0 1.0 0.0 0 0))))

(event EventInternalInteract
  (Rendering|Components|Sprite|SetSprite (Variables|Default|GetPaperSprite) (Variables|Default|GetSourceSpriteActivated))
  (Default|Receive (Variables|Default|GetDoorRef)))

(fn ConstructionScript
  (|CallParentFunction))

(fn CanInteract
  (return true))