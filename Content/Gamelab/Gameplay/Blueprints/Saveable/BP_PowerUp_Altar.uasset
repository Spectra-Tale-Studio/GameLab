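; An interactable power-up altar that alters one player attribute when used, selected by its Type setting.
; Interact gets the player through the GameInstance, then changes max jumps, dash unlock state, max health or current health using the configured values.
; A current-health boost that exceeds the maximum raises max health to match rather than clamping.
; The parent class's Interact runs after the effect is applied.
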(event EventBeginPlay
  (|CallParentFunction) ; This node is disabled and will not be called.\nDrag off pins to build functionality.
)

(event Collision|EventActorBeginOverlap
  (params (OtherActor :type Actor%20Object%20Reference))
  (|CallParentFunction OtherActor) ; This node is disabled and will not be called.\nDrag off pins to build functionality.
)

(event EventTick
  (params (DeltaSeconds :type Float%20%28single-precision%29))
  (|CallParentFunction DeltaSeconds) ; This node is disabled and will not be called.\nDrag off pins to build functionality.
)

(event EventInteract
  (bind _reference (Class|BPIPlayerRef|GetPlayerRef(Message) (Game|GetGameInstance)))
  (Utilities|FlowControl|Sequence
    (:then_0
      (switch Utilities|FlowControl|Switch|SwitchonE_PowerUPType (Variables|Default|GetType)
        (:NewEnumerator0
          (Variables|/Game/Gamelab/Gameplay/Characters/Player/BP_Player.BP_Player_C|SetMaxAvailableJumps _reference (+ (Variables|/Game/Gamelab/Gameplay/Characters/Player/BP_Player.BP_Player_C|GetMaxAvailableJumps _reference) (Math|Float|Truncate (Variables|Default|GetIncrement)))))
        (:NewEnumerator1
          (Variables|/Game/Gamelab/Gameplay/Characters/Player/BP_Player.BP_Player_C|SetDashUnlock _reference (Variables|Default|GetDashUnlock)))
        (:NewEnumerator2
          (Variables|/Game/Gamelab/Gameplay/Blueprints/Health_Component/BP_HealthComponent.BP_HealthComponent_C|SetRuntimeMaxHealth (Variables|/Game/Gamelab/Gameplay/Characters/BP_CharacterBase_PaperZD.BP_CharacterBase_PaperZD_C|GetBP_HealthComponent _reference) (+ (Variables|/Game/Gamelab/Gameplay/Blueprints/Health_Component/BP_HealthComponent.BP_HealthComponent_C|GetRuntimeMaxHealth (Variables|/Game/Gamelab/Gameplay/Characters/BP_CharacterBase_PaperZD.BP_CharacterBase_PaperZD_C|GetBP_HealthComponent _reference)) (Variables|Default|GetIncrement))))
        (:NewEnumerator3
          (if (> (+ (Variables|/Game/Gamelab/Gameplay/Blueprints/Health_Component/BP_HealthComponent.BP_HealthComponent_C|GetCurrentHealth (Variables|/Game/Gamelab/Gameplay/Characters/BP_CharacterBase_PaperZD.BP_CharacterBase_PaperZD_C|GetBP_HealthComponent _reference)) (Variables|Default|GetIncrement)) (Variables|/Game/Gamelab/Gameplay/Blueprints/Health_Component/BP_HealthComponent.BP_HealthComponent_C|GetRuntimeMaxHealth (Variables|/Game/Gamelab/Gameplay/Characters/BP_CharacterBase_PaperZD.BP_CharacterBase_PaperZD_C|GetBP_HealthComponent _reference)))
            (Variables|/Game/Gamelab/Gameplay/Blueprints/Health_Component/BP_HealthComponent.BP_HealthComponent_C|SetRuntimeMaxHealth (Variables|/Game/Gamelab/Gameplay/Characters/BP_CharacterBase_PaperZD.BP_CharacterBase_PaperZD_C|GetBP_HealthComponent _reference) (+ (Variables|/Game/Gamelab/Gameplay/Blueprints/Health_Component/BP_HealthComponent.BP_HealthComponent_C|GetCurrentHealth (Variables|/Game/Gamelab/Gameplay/Characters/BP_CharacterBase_PaperZD.BP_CharacterBase_PaperZD_C|GetBP_HealthComponent _reference)) (Variables|Default|GetIncrement))))
          (Variables|/Game/Gamelab/Gameplay/Blueprints/Health_Component/BP_HealthComponent.BP_HealthComponent_C|SetCurrentHealth (Variables|/Game/Gamelab/Gameplay/Characters/BP_CharacterBase_PaperZD.BP_CharacterBase_PaperZD_C|GetBP_HealthComponent _reference) (+ (Variables|/Game/Gamelab/Gameplay/Blueprints/Health_Component/BP_HealthComponent.BP_HealthComponent_C|GetCurrentHealth (Variables|/Game/Gamelab/Gameplay/Characters/BP_CharacterBase_PaperZD.BP_CharacterBase_PaperZD_C|GetBP_HealthComponent _reference)) (Variables|Default|GetIncrement))))))
    (:then_1
      (|CallParentFunction))))

(fn ConstructionScript
  (|CallParentFunction))