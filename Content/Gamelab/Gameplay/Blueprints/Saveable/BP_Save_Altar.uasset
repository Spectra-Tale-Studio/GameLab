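; BP_Save_Altar is an interactable save point that fully heals the player and saves their progress.
; On Interact, it gets the player through the GameInstance and restores health to the runtime maximum.
; If the save data object is valid, it writes transform, jump count, dash unlock and health into PlayerData, saves through the GameInstance, then calls the parent Interact.
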(event EventBeginPlay
  (|CallParentFunction) ; This node is disabled and will not be called.\nDrag off pins to build functionality.
)

(event Collision|EventActorBeginOverlap
  (params (OtherActor :type Actor%20Object%20Reference))
  (|CallParentFunction OtherActor) ; This node is disabled and will not be called.\nDrag off pins to build functionality.
)

(event EventTick
  (params (DeltaSeconds :type Float%20%28single-precision%29))
  (|CallParentFunction DeltaSeconds) ; This node is disabled and will not be called.\nDrag off pins to build functionality.
)

(event EventInteract
  (bind _returnvalue (Game|GetGameInstance))
  (bind _reference (Class|BPIPlayerRef|GetPlayerRef(Message) _returnvalue))
  (Variables|/Game/Gamelab/Gameplay/Blueprints/Health_Component/BP_HealthComponent.BP_HealthComponent_C|SetCurrentHealth (Variables|/Game/Gamelab/Gameplay/Characters/BP_CharacterBase_PaperZD.BP_CharacterBase_PaperZD_C|GetBP_HealthComponent _reference) (Variables|/Game/Gamelab/Gameplay/Blueprints/Health_Component/BP_HealthComponent.BP_HealthComponent_C|GetRuntimeMaxHealth (Variables|/Game/Gamelab/Gameplay/Characters/BP_CharacterBase_PaperZD.BP_CharacterBase_PaperZD_C|GetBP_HealthComponent _reference)))
  (bind _gamedata (Class|BPISaveGame|GetData(Message) _returnvalue))
  (Utilities|IsValid _gamedata
    (:Is%20Valid
      (Variables|/Game/Developers/AndreaFrigerio/SaveSystem/SG_GameplaySave.SG_GameplaySave_C|SetPlayerData _gamedata (Utilities|Struct|MakeFPlayerSaveData (Transformation|GetActorTransform _reference) (Variables|/Game/Gamelab/Gameplay/Characters/Player/BP_Player.BP_Player_C|GetMaxAvailableJumps _reference) (Variables|/Game/Gamelab/Gameplay/Characters/Player/BP_Player.BP_Player_C|GetDashUnlock _reference) (Variables|/Game/Gamelab/Gameplay/Blueprints/Health_Component/BP_HealthComponent.BP_HealthComponent_C|GetRuntimeMaxHealth (Variables|/Game/Gamelab/Gameplay/Characters/BP_CharacterBase_PaperZD.BP_CharacterBase_PaperZD_C|GetBP_HealthComponent _reference)) (Variables|/Game/Gamelab/Gameplay/Blueprints/Health_Component/BP_HealthComponent.BP_HealthComponent_C|GetRuntimeMaxHealth (Variables|/Game/Gamelab/Gameplay/Characters/BP_CharacterBase_PaperZD.BP_CharacterBase_PaperZD_C|GetBP_HealthComponent _reference))))
      (Class|BPISaveGame|SaveData(Message) _returnvalue)
      (|CallParentFunction))))

(fn ConstructionScript
  (|CallParentFunction))